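; BP_Soul is a soul actor in the Pickups folder that slowly sinks toward the ground and stops at a hover height.
; On BeginPlay, a downward object trace, with debug drawing on, finds the surface below and stores a minimum height slightly above it.
; Tick moves the actor down in local Z at a constant, frame-rate-independent speed while it is above that height.
; It contains no collection logic.
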(event EventBeginPlay
  (bind _returnvalue (Transformation|GetActorLocation))
  (bind _outhit (Collision|LineTraceForObjects _returnvalue (- _returnvalue "0.000000,0.000000,2000.000000") (Variables|Default|GetObject%20TypesArray) false (Utilities|Array|MakeArray (Components|GetOwner)) "ForDuration"))
  (Variables|Default|SetSoulMinHieght (.z (+ (.ImpactPoint (Collision|BreakHitResult _outhit)) "0.000000,0.000000,75.000000"))))

(event EventTick
  (params (DeltaSeconds :type Float%20%28single-precision%29))
  (if (> (.z (Transformation|GetActorLocation)) (Variables|Default|GetSoulMinHieght))
    (Transformation|AddActorLocalOffset (Math|Vector|MakeVector 0.0 0.0 (* DeltaSeconds -2e+01)) false false)))

(fn ConstructionScript)