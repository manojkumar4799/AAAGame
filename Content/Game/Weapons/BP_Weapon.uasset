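; BP_Weapon is a weapon Blueprint that applies Chaos physics fields at a given location to break and scatter destructible objects.
; Its CreateFieldForce event applies external cluster strain through a radial falloff to fracture clusters around that point.
; After a brief delay, it applies a filtered radial-vector linear force to push pieces away, then draws a debug sphere at the location.
; The file contains no firing or hit-detection logic.
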(event EventCreateFieldForce
  (params (fieldForceLocation :type Vector%20%28by%20ref%29 :default "0, 0, 0"))
  (Class|FieldSystemComponent|ApplyPhysicsField (Variables|Default|GetFieldSystem) true "Field_ExternalClusterStrain" 0 (Field|SetRadialFalloff (Variables|Default|GetRadialFalloff) 10000004.0 0.8 1.0 0.0 2e+02 fieldForceLocation "Field_FallOff_None"))
  (Utilities|FlowControl|Delay 0.05)
  (Class|FieldSystemComponent|ApplyPhysicsField (Variables|Default|GetFieldSystem) true "Field_LinearForce" (Variables|Default|GetFieldSystemMetaDataFilter) (Field|SetRadialVector (Variables|Default|GetRadialVector) 4000008.0 fieldForceLocation))
  (Rendering|Debug|DrawDebugSphere fieldForceLocation 1e+01 12 "(R=1.000000,G=1.000000,B=1.000000,A=1.000000)" 1.0))

(fn ConstructionScript)